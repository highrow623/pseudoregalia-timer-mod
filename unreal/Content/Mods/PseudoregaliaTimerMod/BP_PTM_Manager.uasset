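; Manager actor for the Pseudoregalia timer mod that shows a timer widget and mirrors other players as colored, named ghosts.
; Outside the title and end screens, it adds the widget and passes the active room and player transform to SyncInfo each tick.
; UpdateGhosts spawns, teleports or removes ghost actors through an ID-keyed map.
; SyncInfo is an empty stub and UpdateGhosts has no caller here, suggesting external hooks handle the exchange.
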(event `self.ReceiveTick`
  (params (DeltaSeconds :type "Float (single-precision)"))
  (if (`self.Run`)
    (bind _info (`self.MakePlayerInfo`))
    (`self.SyncInfo` (`/Game/Blueprints/GameData/MV_GameInstance.activeRoom` (`self.GameInstanceRef`)) _info)))

(event `self.ReceiveBeginPlay`
  (`|ExecutionSequence`
    (:`then_0`
      (bind (_startindex _endindex) (`/Game/Mods/PseudoregaliaTimerMod/BPL_PTM_Save.GetData`))
      (set `self.StartIndex` _startindex)
      (set `self.EndIndex` _endindex))
    (:`then_1`
      (bind _asmv_game_instance (cast `/Game/Blueprints/GameData/MV_GameInstance` (`GameplayStatics.GetGameInstance`))
        (:`then`
          (set `self.GameInstanceRef` _asmv_game_instance))
        (:`CastFailed`
          (`self.PrintToModLoader` "failed to cast game instance to MV_GameInstance"))))
    (:`then_2`
      (bind _returnvalue (`GameplayStatics.GetActorOfClass` "/Game/ThirdPerson/Player/BP_PlayerGoatMain.BP_PlayerGoatMain_C"))
      (set `self.PlayerRef` _returnvalue))
    (:`then_3`
      (bind _returnvalue_2 (`GameplayStatics.GetCurrentLevelName` true))
      (bind _output_get (set `self.Run` (`KismetMathLibrary.BooleanNOR` (`KismetStringLibrary.EqualEqual_StrStr` _returnvalue_2 "TitleScreen") (`KismetStringLibrary.EqualEqual_StrStr` _returnvalue_2 "EndScreen"))))
      (if _output_get
        (bind _returnvalue_3 (`|CreateWidget` "/Game/Mods/PseudoregaliaTimerMod/Timer/WBP_PTM_Timer.WBP_PTM_Timer_C" (`GameplayStatics.GetPlayerController` 0)))
        (bind _output_get_2 (set `self.TimerWidgetRef` _returnvalue_3))
        (`UserWidget.AddToViewport` _output_get_2 0)))))

(event `PrintToModLoader`
  (params (Message :type String)))

(fn `MakePlayerInfo`
  (returns (Info :type "/Game/Mods/PseudoregaliaTimerMod/ST_PlayerInfo Structure"))
  (bind _returnvalue (`self.GetTransform` (`self.PlayerRef`)))
  (return (make `/Game/Mods/PseudoregaliaTimerMod/ST_PlayerInfo` :`location_x` (.x (.location _returnvalue)) :`location_y` (.y (.location _returnvalue)) :`location_z` (.z (.location _returnvalue)) :`rotation_x` (.roll (.rotation _returnvalue)) :`rotation_y` (.pitch (.rotation _returnvalue)) :`rotation_z` (.yaw (.rotation _returnvalue)))))

(fn `RemoveGhost`
  (params (id :type Byte))
  (bind _ghosts (`self.Ghosts`))
  (`self.K2_DestroyActor` (`BlueprintMapLibrary.Map_Find` _ghosts id))
  (`BlueprintMapLibrary.Map_Remove` _ghosts id))

(fn `SpawnGhost`
  (params (info :type "/Game/Mods/PseudoregaliaTimerMod/ST_PlayerInfo Structure"))
  (bind _returnvalue (`|SpawnActorFromClass` "/Game/Mods/PseudoregaliaTimerMod/BP_PTM_Ghost.BP_PTM_Ghost_C" (`KismetMathLibrary.MakeTransform` (`KismetMathLibrary.MakeVector` info_location_x_47_C9359E5E4979B04BE501BEB2E9214E4E info_location_y_50_8788267F4AE0DCB7D3ACA8B9C327C862 info_location_z_51_08ADD7BB4F7F6896B9136FBA1FC19E49) (`KismetMathLibrary.MakeRotator` info_rotation_x_53_EEAABFEB4AF40672CA6873883323E0A1 info_rotation_y_56_DBEDDCA347AC24CEFDAFBA93176A360B info_rotation_z_57_1D92B39E435E59BFE015F4B729C51619)) "AlwaysSpawn" "OverrideRootScale" null (`KismetMathLibrary.MakeColor` (/ (`KismetMathLibrary.Conv_ByteToDouble` info_red_67_6D737E6F45D30EB007F10E9D890B4ED3) 255.0) (/ (`KismetMathLibrary.Conv_ByteToDouble` info_green_70_07BFE5944C2B4196E09760B0A19BE93C) 255.0) (/ (`KismetMathLibrary.Conv_ByteToDouble` info_blue_71_7E8CED514EA98596E3AAA6A40B06BAE6) 255.0)) 0.6 info_name_76_6BF1519946162D11DFD8759F7E96EB7D null))
  (`BlueprintMapLibrary.Map_Add` (`self.Ghosts`) info_id_64_ACEE325C40A82A6010DF82BF448FD0B6 _returnvalue))

(fn `SyncInfo`
  (params (ActiveRoom :type Integer) (Info :type "/Game/Mods/PseudoregaliaTimerMod/ST_PlayerInfo Structure")))

(fn `TryRemoveGhost`
  (params (id :type Byte))
  (if (`BlueprintMapLibrary.Map_Contains` (`self.Ghosts`) id)
    (`self.RemoveGhost` id)))

(fn `UpdateGhost`
  (params (info :type "/Game/Mods/PseudoregaliaTimerMod/ST_PlayerInfo Structure"))
  (bind ((`location_x_47_C9359E5E4979B04BE501BEB2E9214E4E` _location_x) (`location_y_50_8788267F4AE0DCB7D3ACA8B9C327C862` _location_y) (`location_z_51_08ADD7BB4F7F6896B9136FBA1FC19E49` _location_z) (`rotation_x_53_EEAABFEB4AF40672CA6873883323E0A1` _rotation_x) (`rotation_y_56_DBEDDCA347AC24CEFDAFBA93176A360B` _rotation_y) (`rotation_z_57_1D92B39E435E59BFE015F4B729C51619` _rotation_z) (`id_64_ACEE325C40A82A6010DF82BF448FD0B6` _id)) (break `/Game/Mods/PseudoregaliaTimerMod/ST_PlayerInfo` info))
  (`self.K2_SetActorTransform` (`BlueprintMapLibrary.Map_Find` (`self.Ghosts`) _id) (`KismetMathLibrary.MakeTransform` (`KismetMathLibrary.MakeVector` _location_x _location_y _location_z) (`KismetMathLibrary.MakeRotator` _rotation_x _rotation_y _rotation_z)) false true))

(fn `UpdateGhosts`
  (params (GhostInfo :type "Array of /Game/Mods/PseudoregaliaTimerMod/ST_PlayerInfo Structure") (ToRemove :type "Array of Byte"))
  (locals (ids :type "Set of String"))
  (for _array_element GhostInfo
    (`self.CheckGhost` _array_element
      (:`Exists`
        (`self.UpdateGhost` _array_element))
      (:`Doesn't Exist`
        (`self.SpawnGhost` _array_element))))
  (for _array_element_2 ToRemove
    (`self.TryRemoveGhost` _array_element_2)))

(fn `UserConstructionScript`)