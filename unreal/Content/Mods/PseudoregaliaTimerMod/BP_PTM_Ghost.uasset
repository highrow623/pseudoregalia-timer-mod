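; BP_PTM_Ghost is a ghost actor for the Pseudoregalia timer mod, showing a Sybil mesh with a floating name label.
; On BeginPlay it pushes its Color and Intensity into the mesh's DieColor and DieAmount material parameters to tint it, and sets the label text from Name.
; Each Tick it rotates the text to face the player camera.
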(event `self.ReceiveBeginPlay`
  (bind _sybilmesh (`self.sybilMesh`))
  (`MeshComponent.SetVectorParameterValueOnMaterials` _sybilmesh "DieColor" (`KismetMathLibrary.Conv_LinearColorToVector` (`self.Color`)))
  (`MeshComponent.SetScalarParameterValueOnMaterials` _sybilmesh "DieAmount" (`self.Intensity`))
  (`TextRenderComponent.K2_SetText` (`self.TextRender`) (`KismetTextLibrary.Conv_StringToText` (`self.Name`))))

(event `self.ReceiveTick`
  (params (DeltaSeconds :type "Float (single-precision)"))
  (bind _textrender (`self.TextRender`))
  (`SceneComponent.K2_SetWorldRotation` _textrender (`KismetMathLibrary.FindLookAtRotation` (`SceneComponent.K2_GetComponentLocation` _textrender) (`SceneComponent.K2_GetComponentLocation` (`PlayerCameraManager.TransformComponent` (`GameplayStatics.GetPlayerCameraManager` 0)))) false false))

(fn `UserConstructionScript`)